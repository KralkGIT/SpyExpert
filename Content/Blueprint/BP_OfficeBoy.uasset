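; BP_OfficeBoy is the third-person player character, with Enhanced Input movement, sprinting and weapon combat.
; An overlap detector finds BP_Weapon actors, whose data drives pickup, dropping and swapping between holstered and armed meshes.
; Aiming zooms the spring arm and enables rate-limited line-trace shots that damage BP_Enemy, with montage-driven firing and reloading.
; It also tracks ammo and health, prints both as debug text, and ragdolls on death.
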(event OnComponentBeginOverlap(PickupDetector)
  (params (OverlappedComponent :type Primitive%20Component%20Object%20Reference) (OtherActor :type Actor%20Object%20Reference) (OtherComp :type Primitive%20Component%20Object%20Reference) (OtherBodyIndex :type Integer) (bFromSweep :type Boolean) (SweepResult :type Hit%20Result%20Structure%20%28by%20ref%29))
  (bind _asbp_weapon (Utilities|Casting|CastToBP_Weapon OtherActor))
  (Variables|Default|SetDetectedWeapon _asbp_weapon))

(event OnComponentEndOverlap(PickupDetector)
  (params (OverlappedComponent :type Primitive%20Component%20Object%20Reference) (OtherActor :type Actor%20Object%20Reference) (OtherComp :type Primitive%20Component%20Object%20Reference) (OtherBodyIndex :type Integer))
  (Variables|Default|SetDetectedWeapon 0))

(event Input|EnhancedActionEvents|EnhancedInputActionIA_Aim
  (params (ActionValue :type Boolean) (ElapsedSeconds :type Float%20%28double-precision%29) (TriggeredSeconds :type Float%20%28double-precision%29) (InputAction :type Input%20Action%20Object%20Reference :default "/Game/Character/Input/IA_Aim.IA_Aim"))
  (bind _charactermovement (Variables|Character|GetCharacterMovement))
  (bind _charactermovement_2 (Variables|Character|GetCharacterMovement))
  (:Triggered
    (if (and (Utilities|IsValid (Variables|Default|GetWeapon)) (not (Variables|Default|GetIsWeaponHolster)))
      (Variables|Default|SetIsAiming true)
      (Variables|/Script/Engine.CharacterMovementComponent|SetbUseControllerDesiredRotation _charactermovement_2 true)
      (Variables|/Script/Engine.CharacterMovementComponent|SetbOrientRotationToMovement _charactermovement_2 false)
      (bind _alpha (Timeline|AnimateZoom Play)
        (:Update
          (Variables|/Script/Engine.SpringArmComponent|SetTargetArmLength (Variables|Default|GetSpringArm) (Math|Float|Lerp 3e+02 1e+02 _alpha))))))
  (:Completed
    (Variables|Default|SetIsAiming false)
    (Variables|/Script/Engine.CharacterMovementComponent|SetbUseControllerDesiredRotation _charactermovement false)
    (Variables|/Script/Engine.CharacterMovementComponent|SetbOrientRotationToMovement _charactermovement true)
    (Timeline|AnimateZoom Reverse)))

(event Input|EnhancedActionEvents|EnhancedInputActionIA_Shoot
  (params (ActionValue :type Boolean) (ElapsedSeconds :type Float%20%28double-precision%29) (TriggeredSeconds :type Float%20%28double-precision%29) (InputAction :type Input%20Action%20Object%20Reference :default "/Game/Character/Input/IA_Shoot.IA_Shoot"))
  (bind _armedweaponmesh (Variables|Default|GetArmedWeaponMesh))
  (bind _returnvalue (Transformation|GetSocketLocation _armedweaponmesh "muzzlesocket"))
  (if (and (Variables|Default|GetIsAiming) (> (Variables|Default|GetMagAmmunition) 0))
    (Utilities|FlowControl|Sequence
      (:then_0
        (Utilities|FlowControl|DoOnce false :!label _label
          (:Completed
            (Animation|Montage|PlayMontage (Variables|Character|GetMesh) "/Game/Character/OfficeBoy/Animation/AM_Shoot.AM_Shoot" 0.5
              (:then
                (bind _outhit (Collision|LineTraceByChannel _returnvalue (+ _returnvalue (* (Math|Vector|GetForwardVector (Transformation|GetWorldRotation (Variables|Default|GetSphere))) (Variables|/Game/Weapon/DA_Weapon.DA_Weapon_C|GetFireDistance (Variables|Default|GetWeapon)))) "TraceTypeQuery1" false 0 "ForDuration" true "(R=1.000000,G=0.000000,B=0.000000,A=1.000000)" "(R=0.000000,G=1.000000,B=0.000000,A=1.000000)" 2.0))
                (Variables|Default|SetMagAmmunition (- (Variables|Default|GetMagAmmunition) 1))
                (Development|PrintString (Utilities|GetObjectName (.hitactor _outhit)))
                (bind _asbp_enemy (Utilities|Casting|CastToBP_Enemy (.hitactor _outhit)))
                (Game|Damage|ApplyDamage _asbp_enemy 2e+01 0 0))))))
      (:then_1
        (Utilities|FlowControl|Delay (Variables|/Game/Weapon/DA_Weapon.DA_Weapon_C|GetFireRate (Variables|Default|GetWeapon)))
        (goto _label Reset)))))

(event Input|EnhancedActionEvents|EnhancedInputActionIA_Look
  (params (ActionValue :type Vector%202D%20Structure) (ElapsedSeconds :type Float%20%28double-precision%29) (TriggeredSeconds :type Float%20%28double-precision%29) (InputAction :type Input%20Action%20Object%20Reference :default "/Game/Character/Input/IA_Look.IA_Look"))
  (Pawn|Input|AddControllerYawInput (.x ActionValue))
  (Pawn|Input|AddControllerPitchInput (.y ActionValue)))

(event Input|EnhancedActionEvents|EnhancedInputActionIA_Movement
  (params (ActionValue :type Vector%202D%20Structure) (ElapsedSeconds :type Float%20%28double-precision%29) (TriggeredSeconds :type Float%20%28double-precision%29) (InputAction :type Input%20Action%20Object%20Reference :default "/Game/Character/Input/IA_Movement.IA_Movement"))
  (bind _returnvalue (Pawn|GetControlRotation :!class /Script/Engine.Pawn))
  (Pawn|Input|AddMovementInput (Math|Vector|GetRightVector (Pawn|GetControlRotation :!class /Script/Engine.Pawn)) (.x ActionValue) false)
  (Pawn|Input|AddMovementInput (Math|Vector|GetForwardVector (Math|Rotator|MakeRotator (.roll _returnvalue) 0.0 (.yaw _returnvalue))) (.y ActionValue) false))

(event Input|EnhancedActionEvents|EnhancedInputActionIA_Sprint
  (params (ActionValue :type Boolean) (ElapsedSeconds :type Float%20%28double-precision%29) (TriggeredSeconds :type Float%20%28double-precision%29) (InputAction :type Input%20Action%20Object%20Reference :default "/Game/Character/Input/IA_Sprint.IA_Sprint"))
  (bind _charactermovement (Variables|Character|GetCharacterMovement))
  (:Started
    (Variables|/Script/Engine.CharacterMovementComponent|SetMaxWalkSpeed _charactermovement (Variables|Default|GetSprintSpeed)))
  (:Completed
    (Variables|/Script/Engine.CharacterMovementComponent|SetMaxWalkSpeed _charactermovement (Variables|Default|GetWalkingSpeed))))

(event Input|EnhancedActionEvents|EnhancedInputActionIA_PickUp
  (params (ActionValue :type Boolean) (ElapsedSeconds :type Float%20%28double-precision%29) (TriggeredSeconds :type Float%20%28double-precision%29) (InputAction :type Input%20Action%20Object%20Reference :default "/Game/Character/Input/IA_PickUp.IA_PickUp"))
  (:Started
    (Utilities|PickupWeapon)))

(event Input|EnhancedActionEvents|EnhancedInputActionIA_Drop
  (params (ActionValue :type Boolean) (ElapsedSeconds :type Float%20%28double-precision%29) (TriggeredSeconds :type Float%20%28double-precision%29) (InputAction :type Input%20Action%20Object%20Reference :default "/Game/Character/Input/IA_Drop.IA_Drop"))
  (:Started
    (Utilities|DropWeapon)))

(event Input|EnhancedActionEvents|EnhancedInputActionIA_Holster
  (params (ActionValue :type Boolean) (ElapsedSeconds :type Float%20%28double-precision%29) (TriggeredSeconds :type Float%20%28double-precision%29) (InputAction :type Input%20Action%20Object%20Reference :default "/Game/Character/Input/IA_Holster.IA_Holster"))
  (:Started
    (Utilities|IsValid (Variables|Default|GetWeapon)
      (:Is%20Valid
        (if (Variables|Default|GetIsWeaponHolster)
          (Variables|Default|SetIsWeaponHolster false)
          (Components|SkeletalMesh|SetSkeletalMeshAsset (Variables|Default|GetHoslterWeaponMesh) 0)
          (Components|SkeletalMesh|SetSkeletalMeshAsset (Variables|Default|GetArmedWeaponMesh) (Variables|/Game/Weapon/DA_Weapon.DA_Weapon_C|GetMesh (Variables|Default|GetWeapon)))
          (else
            (Variables|Default|SetIsWeaponHolster true)
            (Components|SkeletalMesh|SetSkeletalMeshAsset (Variables|Default|GetHoslterWeaponMesh) (Variables|/Game/Weapon/DA_Weapon.DA_Weapon_C|GetMesh (Variables|Default|GetWeapon)))
            (Components|SkeletalMesh|SetSkeletalMeshAsset (Variables|Default|GetArmedWeaponMesh) 0)))))))

(event Input|EnhancedActionEvents|EnhancedInputActionIA_Reload
  (params (ActionValue :type Boolean) (ElapsedSeconds :type Float%20%28double-precision%29) (TriggeredSeconds :type Float%20%28double-precision%29) (InputAction :type Input%20Action%20Object%20Reference :default "/Game/Character/Input/IA_Reload.IA_Reload"))
  (:Started
    (if (and (< (Variables|Default|GetMagAmmunition) (Variables|/Game/Weapon/DA_Weapon.DA_Weapon_C|GetMaxMagazine (Variables|Default|GetWeapon))) (> (Variables|Default|GetTotalAmmunition) 0))
      (Animation|Montage|PlayMontage (Variables|Character|GetMesh) "/Game/Character/OfficeBoy/Animation/AM_ReloadRifle.AM_ReloadRifle"
        (:OnCompleted
          (if (>= (Variables|Default|GetTotalAmmunition) (- (Variables|/Game/Weapon/DA_Weapon.DA_Weapon_C|GetMaxMagazine (Variables|Default|GetWeapon)) (Variables|Default|GetMagAmmunition)))
            (Variables|Default|SetTotalAmmunition (- (Variables|Default|GetTotalAmmunition) (- (Variables|/Game/Weapon/DA_Weapon.DA_Weapon_C|GetMaxMagazine (Variables|Default|GetWeapon)) (Variables|Default|GetMagAmmunition))))
            (Variables|Default|SetMagAmmunition (+ (Variables|Default|GetMagAmmunition) (- (Variables|/Game/Weapon/DA_Weapon.DA_Weapon_C|GetMaxMagazine (Variables|Default|GetWeapon)) (Variables|Default|GetMagAmmunition))))
            (else
              (Variables|Default|SetMagAmmunition (+ (Variables|Default|GetMagAmmunition) (Variables|Default|GetTotalAmmunition)))
              (Variables|Default|SetTotalAmmunition (- (Variables|Default|GetTotalAmmunition) (Variables|Default|GetTotalAmmunition))))))))))

(event EventBeginPlay
  (bind _asbp_tpscontroller (Utilities|Casting|CastToBP_TPSController (Pawn|GetController)))
  (Input|AddMappingContext (PlayerController|LocalPlayerSubsystems|GetEnhancedInputLocalPlayerSubsystem _asbp_tpscontroller) "/Game/Character/Input/IMP_Char.IMP_Char" 0 "(bIgnoreAllPressedKeysUntilRelease=True,bForceImmediately=False,bNotifyUserSettings=False)")
  (Variables|/Script/Engine.CharacterMovementComponent|SetMaxWalkSpeed (Variables|Character|GetCharacterMovement) (Variables|Default|GetWalkingSpeed))
  (Variables|Default|SetHealth (Variables|Default|GetMaxHealth)))

(event EventTick
  (params (DeltaSeconds :type Float%20%28single-precision%29))
  (Development|PrintString (Utilities|String|Append (Utilities|String|ToString(Integer) (Variables|Default|GetMagAmmunition)) "/" (Utilities|String|ToString(Integer) (Variables|Default|GetTotalAmmunition))) true true "(R=0.000000,G=0.660000,B=1.000000,A=1.000000)" 0.01)
  (Development|PrintString (Utilities|String|Append "Player Health: " (Utilities|String|ToString(Integer) (Variables|Default|GetHealth)) "/" (Utilities|String|ToString(Integer) (Variables|Default|GetMaxHealth))) true true "(R=0.000000,G=0.660000,B=1.000000,A=1.000000)" 0.01))

(event Game|Damage|EventAnyDamage
  (params (Damage :type Float%20%28single-precision%29) (DamageType :type Damage%20Type%20Object%20Reference) (InstigatedBy :type Controller%20Object%20Reference) (DamageCauser :type Actor%20Object%20Reference))
  (if (not (Variables|Default|GetIsDeath?))
    (Variables|Default|SetHealth (- (Variables|Default|GetHealth) Damage))
    (if (<= (Variables|Default|GetHealth) 0)
      (Variables|Default|SetIsDeath? true)
      (Physics|SetSimulatePhysics (Variables|Character|GetMesh) true))))

(fn ConstructionScript)

(fn AddHealth
  (params (HealthToAdd :type Integer))
  (Variables|Default|SetHealth (+ (Variables|Default|GetHealth) HealthToAdd))
  (if (> (Variables|Default|GetHealth) (Variables|Default|GetMaxHealth))
    (Variables|Default|SetMaxHealth (Variables|Default|GetMaxHealth))))

(fn AddAmmunition
  (params (AmmunitionToAdd :type Integer))
  (Variables|Default|SetTotalAmmunition (+ (Variables|Default|GetTotalAmmunition) AmmunitionToAdd))
  (if (> (Variables|Default|GetTotalAmmunition) (Variables|/Game/Weapon/DA_Weapon.DA_Weapon_C|GetMaxAmmunition (Variables|Default|GetWeapon)))
    (Variables|Default|SetTotalAmmunition (Variables|/Game/Weapon/DA_Weapon.DA_Weapon_C|GetMaxAmmunition (Variables|Default|GetWeapon)))))