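; BP_Enemy is an AI enemy that patrols random nearby points, then chases and shoots BP_OfficeBoy when Pawn Sensing sees it.
; Each sighting triggers a move, a snap-turn toward the player and a montage-backed line-trace shot, rate-limited by DoOnce and Delay.
; Weapon data supplies mesh, range and fire rate.
; At zero health it ragdolls and spawns BP_Ammunition; Tick prints health for debugging.
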(event OnSeePawn(PawnSensing)
  (params (Pawn :type Pawn%20Object%20Reference))
  (bind _asbp_office_boy (Utilities|Casting|CastToBP_OfficeBoy Pawn))
  (Variables|Default|SetIsChasing? true)
  (CallFunction|ChasePlayer _asbp_office_boy))

(event Custom|Patrol
  (if (not (Variables|Default|GetIsDeath?))
    (AI|AIMoveTo self (.RandomLocation (AI|Navigation|GetRandomReachablePointinRadius (Transformation|GetActorLocation) 5e+02 0 0)) 0 5.0 false
      (:OnSuccess
        _)
      (:OnFail
        _))
    (Utilities|FlowControl|Delay 2.0)
    (if (not (Variables|Default|GetIsChasing?))
      (CallFunction|Patrol))))

(event Custom|ChasePlayer
  (params (OfficeBoy :type Pawn%20Object%20Reference))
  (if (not (Variables|Default|GetIsDeath?))
    (AI|AIMoveTo self "0, 0, 0" OfficeBoy 5e+01 false
      (:then
        _)
      (:OnSuccess
        (Variables|Default|SetIsChasing? false :!label _label))
      (:OnFail
        (goto _label)))
    (Transformation|SetActorRotation (Math|Rotator|FindLookatRotation (Transformation|GetActorLocation) (Transformation|GetActorLocation OfficeBoy)))
    (CallFunction|Shoot)))

(event Custom|Shoot
  (bind _weaponmesh (Variables|Default|GetWeaponMesh))
  (bind _returnvalue (Transformation|GetSocketLocation _weaponmesh "muzzlesocket"))
  (Utilities|FlowControl|Sequence
    (:then_0
      (Utilities|FlowControl|DoOnce false :!label _label
        (:Completed
          (Animation|Montage|PlayMontage (Variables|Character|GetMesh) "/Game/Character/Enemy/WhiteClown/Animation/AM_WhiteClownShoot.AM_WhiteClownShoot"
            (:then
              (bind _outhit (Collision|LineTraceByChannel _returnvalue (+ (* (Math|Vector|GetForwardVector (Transformation|GetActorRotation)) (Variables|/Game/Weapon/DA_Weapon.DA_Weapon_C|GetFireDistance (Variables|Default|GetWeapon))) _returnvalue) "TraceTypeQuery1" false 0 "ForDuration"))
              (bind _asbp_office_boy (Utilities|Casting|CastToBP_OfficeBoy (.hitactor _outhit)))
              (Game|Damage|ApplyDamage _asbp_office_boy 1e+01 0 0))))))
    (:then_1
      (Utilities|FlowControl|Delay (Variables|/Game/Weapon/DA_Weapon.DA_Weapon_C|GetFireRate (Variables|Default|GetWeapon)))
      (goto _label Reset))))

(event Game|Damage|EventAnyDamage
  (params (Damage :type Float%20%28single-precision%29) (DamageType :type Damage%20Type%20Object%20Reference) (InstigatedBy :type Controller%20Object%20Reference) (DamageCauser :type Actor%20Object%20Reference))
  (if (not (Variables|Default|GetIsDeath?))
    (Variables|Default|SetHealth (- (Variables|Default|GetHealth) Damage))
    (if (<= (Variables|Default|GetHealth) 0)
      (Variables|Default|SetIsDeath? true)
      (Physics|SetSimulatePhysics (Variables|Character|GetMesh) true)
      (Game|SpawnActorfromClass "/Game/Item/BP_Ammunition.BP_Ammunition_C" (Math|Transform|MakeTransform (Transformation|GetActorLocation) "0, 0, 0" "1.000000,1.000000,1.000000") "Undefined" "MultiplyWithRoot" 0 0))))

(event EventTick
  (params (DeltaSeconds :type Float%20%28single-precision%29))
  (Development|PrintString (Utilities|String|Append "Enemy Health: " (Utilities|String|ToString(Integer) (Variables|Default|GetHealth))) true true "(R=0.000000,G=0.660000,B=1.000000,A=1.000000)" 0.001))

(event EventBeginPlay
  (CallFunction|Patrol))

(fn ConstructionScript
  (Components|SkeletalMesh|SetSkeletalMeshAsset (Variables|Default|GetWeaponMesh) (Variables|/Game/Weapon/DA_Weapon.DA_Weapon_C|GetMesh (Variables|Default|GetWeapon))))